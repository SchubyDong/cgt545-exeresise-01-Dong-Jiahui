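; Inside_Door is an automatic swinging door that opens while the third-person player character stands inside its sensor.
; Sensor overlap begin and end events, filtered by a cast to BP_ThirdPersonCharacter, set the SensorDetected flag.
; Tick reads that flag and rotates DoorFrame in fixed, frame-rate-dependent yaw steps toward a quarter turn open or back closed.
; IfOpenNormally selects whether the door swings in positive or negative yaw.
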(event `self.ReceiveTick`
  (params (DeltaSeconds :type "Float (single-precision)"))
  (bind (_relativerotation_roll _relativerotation_pitch _relativerotation_yaw) (`KismetMathLibrary.BreakRotator` (`SceneComponent.RelativeRotation` (`self.Door_Frame`))))
  (bind (_relativerotation_roll_2 _relativerotation_pitch_2 _relativerotation_yaw_2) (`KismetMathLibrary.BreakRotator` (`SceneComponent.RelativeRotation` (`self.Door_Frame`))))
  (bind (_relativerotation_roll_3 _relativerotation_pitch_3 _relativerotation_yaw_3) (`KismetMathLibrary.BreakRotator` (`SceneComponent.RelativeRotation` (`self.Door_Frame`))))
  (bind (_relativerotation_roll_4 _relativerotation_pitch_4 _relativerotation_yaw_4) (`KismetMathLibrary.BreakRotator` (`SceneComponent.RelativeRotation` (`self.Door_Frame`))))
  (if (`self.If_Open_Normally`)
    ;[1 1 1] Open/Close
    (if (`self.Sensor_Detected`)
      (if (<= _relativerotation_yaw 90.0)
        (`SceneComponent.K2_AddRelativeRotation` (`self.Door_Frame`) (struct :`Yaw` 3.0) false false))
      (elif (>= _relativerotation_yaw_2 0.0)
        (`SceneComponent.K2_AddRelativeRotation` (`self.Door_Frame`) (struct :`Yaw` -3.0) false false)))
    (elif (`self.Sensor_Detected`)
      (if (>= _relativerotation_yaw_4 -90.0)
        (`SceneComponent.K2_AddRelativeRotation` (`self.Door_Frame`) (struct :`Yaw` -3.0) false false))
      (elif (<= _relativerotation_yaw_3 0.0)
        (`SceneComponent.K2_AddRelativeRotation` (`self.Door_Frame`) (struct :`Yaw` 3.0) false false)))))

(event `self.Sensor.OnComponentBeginOverlap`
  (params (OverlappedComponent :type "PrimitiveComponent Object Reference") (OtherActor :type "Actor Object Reference") (OtherComp :type "PrimitiveComponent Object Reference") (OtherBodyIndex :type Integer) (bFromSweep :type Boolean) (SweepResult :type "HitResult Structure (by ref)"))
  (cast `/Game/ThirdPerson/Blueprints/BP_ThirdPersonCharacter` OtherActor)
  (set `self.Sensor_Detected` true))

(event `self.Sensor.OnComponentEndOverlap`
  (params (OverlappedComponent :type "PrimitiveComponent Object Reference") (OtherActor :type "Actor Object Reference") (OtherComp :type "PrimitiveComponent Object Reference") (OtherBodyIndex :type Integer))
  (cast `/Game/ThirdPerson/Blueprints/BP_ThirdPersonCharacter` OtherActor)
  (set `self.Sensor_Detected` false))

(fn `UserConstructionScript`)